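; Save game object that captures and restores the player's organ progress, inventory and experience.
; PreSave stores unlocked organs, inventory slots, the hotkeyed organ per organ type, truncated EXP from the ability system and the active organ name.
; PostLoad pushes these back through the progress manager, inventory component and user organ settings, applies EXP as an attribute modifier, then sets the active organ.
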(fn PreSave
  (params (PlayerCharacter :type Character%20Object%20Reference))
  (bind _returnvalue (Class|UserOrganSettings|GetUserOrganSettings))
  (Variables|Default|SetUnlockedOrgans (Class|ProgressManagerSubsystem|GetUnlockedOrgans (Class|ProgressManagerSubsystem|GetProgressManager PlayerCharacter)))
  (Variables|Default|SetInventory (Class|InventoryComponent|GetInventorySlots (Actor|GetComponentbyClass PlayerCharacter "/Script/InventorySystem.InventoryComponent")))
  (bind _enumvalue (|ForEachEOrganType)
    (:LoopBody
      (Utilities|Map|Add (Variables|Default|GetEquippedOrgans) _enumvalue (Class|UserOrganSettings|GetHotKeyOrgan _returnvalue _enumvalue)))
    (:then
      (Variables|Default|SetEXP (Math|Float|Truncate (.ReturnValue (Class|AbilitySystemComponent|GetGameplayAttributeValue (Ability|GetAbilitySystemComponent PlayerCharacter) "(AttributeName=\"Experience\",Attribute=/Script/OrganMechanics.CharacterAttributeSet:Experience,AttributeOwner=\"/Script/CoreUObject.Class'/Script/OrganMechanics.CharacterAttributeSet'\")"))))
      (bind _asorgans_character (Utilities|Casting|CastToOrgansCharacter PlayerCharacter))
      (Variables|Default|SetEquippedOrgan (Class|OrgansCharacter|GetActiveOrganName _asorgans_character)))))

(fn PostLoad
  (params (PlayerCharacter :type Character%20Object%20Reference))
  (bind _returnvalue (Class|UserOrganSettings|GetUserOrganSettings))
  (for _array_element (Variables|Default|GetUnlockedOrgans)
    (Class|ProgressManagerSubsystem|UnlockOrgan (Class|ProgressManagerSubsystem|GetProgressManager PlayerCharacter) _array_element))
  (Class|InventoryComponent|SetInventorySlots (Actor|GetComponentbyClass PlayerCharacter "/Script/InventorySystem.InventoryComponent") (Variables|Default|GetInventory))
  (bind _keys (Utilities|Map|Keys (Variables|Default|GetEquippedOrgans)))
  (for _array_element_2 _keys
    (Class|UserOrganSettings|SetOrganHotKey _returnvalue _array_element_2 (.Value (Utilities|Map|Find (Variables|Default|GetEquippedOrgans) _array_element_2)) PlayerCharacter))
  (Class|GameplayEffectExtender|ApplyModifier (Ability|GetAbilitySystemComponent PlayerCharacter) "(AttributeName=\"Experience\",Attribute=/Script/OrganMechanics.CharacterAttributeSet:Experience,AttributeOwner=\"/Script/CoreUObject.Class'/Script/OrganMechanics.CharacterAttributeSet'\")" (Math|Conversions|ToFloat(Integer) (Variables|Default|GetEXP)))
  (bind _asorgans_character (Utilities|Casting|CastToOrgansCharacter PlayerCharacter))
  (Class|OrgansCharacter|SetActiveOrgan _asorgans_character (Variables|Default|GetEquippedOrgan)))