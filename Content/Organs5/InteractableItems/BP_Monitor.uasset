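; BP_Monitor is an interactable monitor prop that switches to a random colour when used.
; BeginPlay creates a dynamic material instance on the second material slot of its static mesh.
; Interact calls SetColour, which writes a random entry from the Colours array to the material's Colour parameter.
; Its interaction functions report it as always usable, instant and single-shot.
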(event EventBeginPlay
  (bind _returnvalue (Rendering|Material|CreateDynamicMaterialInstance (Variables|Default|GetStaticMesh4) 1 0 "None" :!class /Script/Engine.PrimitiveComponent))
  (Variables|Default|SetDynamicMaterialInstance _returnvalue))

(fn ConstructionScript)

(fn SetColour
  (bind _colours (Variables|Default|GetColours))
  (Rendering|Material|SetVectorParameterValue (Variables|Default|GetDynamicMaterialInstance) "Colour" (Utilities|Array|Get(acopy) _colours (Math|Random|RandomInteger (Utilities|Array|Length _colours))) :!class /Script/Engine.MaterialInstanceDynamic))

(fn CanUserInteract
  (return true))

(fn GetInteractionTime
  (return 0.0))

(fn Interact
  (CallFunction|SetColour)
  (return true))

(fn IsSingleShotInteraction
  (return true))

(fn StopInteract
  (return false))