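; Lock-on component that turns its owning actor to face a locked target.
; Lock runs a near-zero-length sphere trace around the owner for Pawn objects, storing the hit actor as Target or clearing it on a miss, with debug drawing enabled.
; Each Tick, while Target is valid, the owner's yaw snaps toward it, keeping pitch and roll.
; GetData is an empty stub.
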(event EventTick
  (params (DeltaSeconds :type Float%20%28single-precision%29))
  (bind _returnvalue (Components|GetOwner))
  (bind _target (Variables|Default|GetTarget))
  (bind _returnvalue_2 (Transformation|GetActorRotation _returnvalue))
  (Utilities|IsValid _target
    (:Is%20Valid
      (Transformation|SetActorRotation _returnvalue (Math|Rotator|MakeRotator (.roll _returnvalue_2) (.pitch _returnvalue_2) (.yaw (Math|Rotator|FindLookatRotation (Transformation|GetActorLocation _returnvalue) (Transformation|GetActorLocation _target))))))))

(fn Lock
  (bind _returnvalue (Components|GetOwner))
  (bind _returnvalue_2 (Transformation|GetActorLocation _returnvalue))
  (bind (_x _y _z) (Math|Vector|BreakVector _returnvalue_2))
  (bind _outhit (Collision|SphereTraceForObjects _returnvalue_2 (Math|Vector|MakeVector (+ _x 0.1) (+ _y 0.1) (+ _z 0.1)) 7.5e+02 (Utilities|Array|MakeArray "ObjectTypeQuery3") false 0 "ForDuration"))
  (if (.bblockinghit _outhit)
    (Variables|Default|SetTarget (.hitactor _outhit))
    (else
      (Variables|Default|SetTarget 0))))

(fn GetData
  (return 0))