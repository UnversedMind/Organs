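; BP_Chest is an interactable storage chest that opens an inventory transfer menu between the player and its own inventory.
; Interact lazily creates and reuses a WB_AddItemToInventory widget fed both inventories, shows the cursor, blocks look/move input and focuses the menu.
; StopInteract removes the widget, hides the cursor and re-enables movement and look, without resetting the input mode.
; GetData exposes the chest's name and description through property bridges.
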(fn ConstructionScript)

(fn CanUserInteract
  (return true))

(fn GetControls
  (return 0))

(fn GetData
  (bind _returnvalue (Class|StringPropertyBridge|CreatePropertyBridge (Utilities|String|ToString(Text) (Variables|Default|GetInteractableName))))
  (bind _returnvalue_2 (Class|StringPropertyBridge|CreatePropertyBridge (Utilities|String|ToString(Text) (Variables|Default|GetInteractableDescription))))
  (bind _returnvalue_3 (Class|ArrayPropertyBridge|CreatePropertyBridge (Utilities|Array|MakeArray _returnvalue _returnvalue_2)))
  (return _returnvalue_3))

(fn GetInteractionTime
  (return 0.0))

(fn Interact
  (bind _returnvalue (Game|GetPlayerController 0))
  (Variables|/Script/Engine.PlayerController|SetbShowMouseCursor _returnvalue true)
  (Input|SetIgnoreLookInput _returnvalue true)
  (Input|SetIgnoreMoveInput _returnvalue true)
  (Utilities|IsValid (Variables|Default|GetMenu)
    (:Is%20Valid
      _)
    (:Is%20Not%20Valid
      (bind _returnvalue_2 (UserInterface|CreateWidget "/ItemDatabase/Inventory/WB_AddItemToInventory.WB_AddItemToInventory_C" 0 (Actor|GetComponentbyClass (Game|GetPlayerCharacter 0) "/Script/InventorySystem.InventoryComponent") (Variables|Default|GetInventory)))
      (Variables|Default|SetMenu _returnvalue_2)))
  (UserInterface|Viewport|AddtoViewport (Variables|Default|GetMenu) 0)
  (Input|SetInputModeGameandUI (Game|GetPlayerController 0) (Variables|Default|GetMenu) "DoNotLock" false false)
  (return true))

(fn IsSingleShotInteraction
  (return false))

(fn StopInteract
  (bind _returnvalue (Game|GetPlayerController 0))
  (Widget|RemovefromParent (Variables|Default|GetMenu))
  (Variables|/Script/Engine.PlayerController|SetbShowMouseCursor _returnvalue false)
  (Input|SetIgnoreLookInput _returnvalue false)
  (Input|ResetIgnoreMoveInput _returnvalue)
  (return true))