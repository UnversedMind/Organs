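; BP_Save is an interactable save point that saves the game when the player uses it.
; Interacting instantly creates a BP_SaveGame, runs its PreSave on the player character, then writes it asynchronously to a single fixed slot.
; System notifications show progress and completion, while IsSaving blocks further interaction until the write completes.
; Its interaction functions expose name and description through property bridges.
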(event Custom|OnInteract
  (bind _returnvalue (Subsystems|GetNotificationManagerSubsystem))
  (Variables|Default|SetbIsSaving true)
  (Class|NotificationManagerSubsystem|AddNotification (Subsystems|GetNotificationManagerSubsystem) "System" "SAVING IN PROGRESS")
  (bind _returnvalue_2 (SaveGame|CreateSaveGameObject "/Game/Organs5/SaveData/BP_SaveGame.BP_SaveGame_C"))
  (Default|PreSave _returnvalue_2 (Game|GetPlayerCharacter 0))
  (|AsyncSaveGametoSlot self _returnvalue_2 "SaveGame"
    (:Completed
      (Variables|Default|SetbIsSaving false)
      (Class|NotificationManagerSubsystem|RemoveNotification _returnvalue "System")
      (Class|NotificationManagerSubsystem|AddNotification _returnvalue "System" "SAVE COMPLETE"))))

(fn ConstructionScript)

(fn CanUserInteract
  (return (not (Variables|Default|GetbIsSaving))))

(fn GetControls
  (return 0))

(fn GetData
  (bind _returnvalue (Class|StringPropertyBridge|CreatePropertyBridge (Utilities|String|ToString(Text) (Variables|Default|GetInteractableName))))
  (bind _returnvalue_2 (Class|StringPropertyBridge|CreatePropertyBridge (Utilities|String|ToString(Text) (Variables|Default|GetInteractableDescription))))
  (bind _returnvalue_3 (Class|ArrayPropertyBridge|CreatePropertyBridge (Utilities|Array|MakeArray _returnvalue _returnvalue_2)))
  (return _returnvalue_3))

(fn GetInteractionTime
  (return 0.0))

(fn Interact
  (CallFunction|OnInteract)
  (return true))

(fn IsSingleShotInteraction
  (return true))

(fn StopInteract
  (return false))