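; Interactable hinged door that toggles open and closed with an instant, single-shot interaction.
; The OpenDoor timeline plays or reverses to lerp the rotation point's yaw between zero and DoorAngleOnOpen.
; With an InteractionTrigger assigned, direct interaction is disabled and BeginPlay binds an event to that trigger's successful interaction through InteractionEventSubsystem and the player's InteractionController.
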(event EventBeginPlay
  (bind _returnvalue (Game|GetPlayerCharacter 0))
  (bind _interactiontrigger (Variables|Default|GetInteractionTrigger))
  (|CallParentFunction)
  (Utilities|IsValid _interactiontrigger
    (:Is%20Valid
      (Utilities|IsValid _returnvalue
        (:Is%20Valid
          (Class|InteractionEventSubsystem|BindEventtoObjectInteraction (Subsystems|GetInteractionEventSubsystem) (Actor|GetComponentbyClass _returnvalue "/Script/InteractionSystem.InteractionController") _interactiontrigger (EventDispatchers|CreateEvent :!event DoorInteraction)))))))

(fn ConstructionScript)

(fn DoorInteraction
  (bind _opendoor (Variables|Default|GetOpenDoor))
  (if (Variables|Default|GetisOpen)
    (Utilities|String|Reverse _opendoor)
    (else
      (Audio|Components|Audio|Play _opendoor)))
  (Variables|Default|SetisOpen (not (Variables|Default|GetisOpen))))

(fn CanUserInteract
  (return (not (Utilities|IsValid (Variables|Default|GetInteractionTrigger)))))

(fn GetInteractionTime
  (return 0.0))

(fn Interact
  (CallFunction|DoorInteraction)
  (return true))

(fn IsSingleShotInteraction
  (return true))

(fn StopInteract
  (return false))