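; Base weapon actor attached to a character, with mesh and tint chosen by organ name.
; On BeginPlay it binds to the character's organ-name change and to start and stop interaction events for OrganBase.
; Interaction start clears the hit list and enables Tick, which stop disables.
; Each tick sphere-traces for pawns at a mesh socket, ignoring the owner and sending one hit message per actor per interaction.
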(event EventBeginPlay
  (bind _returnvalue (Actor|GetAttachParentActor))
  (bind _returnvalue_2 (Subsystems|GetInteractionEventSubsystem))
  (bind _returnvalue_3 (Actor|GetComponentbyClass _returnvalue "/Script/InteractionSystem.InteractionController"))
  (|CallParentFunction)
  (bind _asorgans_character (Utilities|Casting|CastToOrgansCharacter _returnvalue)
    (:then
      (EventDispatchers|BindEventtoOnOrganNameChanged _asorgans_character (EventDispatchers|CreateEvent :!event SetStaticMesh)))
    (:CastFailed
      _))
  (Class|InteractionEventSubsystem|BindEventtoClassInteraction _returnvalue_2 _returnvalue_3 "/Script/OrganMechanics.OrganBase" (EventDispatchers|CreateEvent :!event OnInteract))
  (Class|InteractionEventSubsystem|BindEventtoClassStopInteraction _returnvalue_2 _returnvalue_3 "/Script/OrganMechanics.OrganBase" (EventDispatchers|CreateEvent :!event OnStopInteract)))

(event EventTick
  (params (DeltaSeconds :type Float%20%28single-precision%29))
  (CallFunction|IsHittingItem))

(fn ConstructionScript)

(fn SetStaticMesh
  (params (OrganName :type Name))
  (Components|StaticMesh|SetStaticMesh (Variables|Default|GetStaticMesh) (Class|OrganSettings|GetWeaponMesh OrganName))
  (bind _returnvalue (Rendering|Material|CreateDynamicMaterialInstance (Variables|Default|GetStaticMesh) 0 0 "None" :!class /Script/Engine.PrimitiveComponent))
  (Rendering|Material|SetVectorParameterValue _returnvalue "Colour" (Class|OrganSettings|GetImageTint OrganName) :!class /Script/Engine.MaterialInstanceDynamic))

(fn OnInteract
  (Utilities|Array|Clear (Variables|Default|GetHit%20Actors))
  (Actor|Tick|SetActorTickEnabled true))

(fn OnStopInteract
  (Actor|Tick|SetActorTickEnabled false))

(fn IsHittingItem
  (bind _staticmesh (Variables|Default|GetStaticMesh))
  (bind _hit_actors (Variables|Default|GetHit%20Actors))
  (bind _returnvalue (Transformation|GetSocketLocation _staticmesh "CheckOnHit"))
  (bind (_outhits _returnvalue_2) (Collision|MultiSphereTraceForObjects _returnvalue _returnvalue (Variables|Default|GetHitRange) (Utilities|Array|MakeArray "ObjectTypeQuery3") false (Utilities|Array|MakeArray (Actor|GetAttachParentActor)) "None" true "(R=1.000000,G=0.000000,B=0.000000,A=1.000000)" "(R=0.000000,G=1.000000,B=0.000000,A=1.000000)" 1.0))
  (if _returnvalue_2
    (for _array_element _outhits
      (if (not (Utilities|Array|ContainsItem _hit_actors (.HitActor (Collision|BreakHitResult _array_element))))
        (Class|OnHit|OnHit(Message) (.HitActor (Collision|BreakHitResult _array_element)))
        (Utilities|Array|Add _hit_actors (.HitActor (Collision|BreakHitResult _array_element)))))))