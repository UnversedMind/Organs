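; Base enemy character Blueprint that takes hits through the Gameplay Ability System and rewards the player with EXP on death.
; BeginPlay binds to the attribute set's character-died event and makes itself the owning actor of its health bar widget.
; OnHit applies a fixed base damage divided by EnemDefence as a negative attribute modifier.
; OnDead adds EXPGained to an attribute on the player's ability system, then destroys the actor.
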(event EventBeginPlay
  (EventDispatchers|BindEventtoCharacterDied (Class|CharacterBase|GetCharacterAttributeSet) (EventDispatchers|CreateEvent :!event OnDead))
  (bind _aswb_enemy_health (Utilities|Casting|CastToWB_EnemyHealth (UserInterface|GetUserWidgetObject (Variables|Default|GetHealthBar))))
  (Variables|/Game/Organs5/UI/Enemy/WB_EnemyHealth.WB_EnemyHealth_C|SetOwningActor _aswb_enemy_health self))

(event EventOnHit
  (Class|GameplayEffectExtender|ApplyModifier (Ability|GetAbilitySystemComponent 0) "(AttributeName=\"Health\",Attribute=/Script/OrganMechanics.CharacterAttributeSet:Health,AttributeOwner=\"/Script/CoreUObject.Class'/Script/OrganMechanics.CharacterAttributeSet'\")" (- 0.0 (/ 5e+01 (Variables|Default|GetEnemDefence)))))

(fn ConstructionScript)

(fn OnDead
  (Class|GameplayEffectExtender|ApplyModifier (Ability|GetAbilitySystemComponent (Game|GetPlayerCharacter 0)) "(AttributeName=\"Experience\",Attribute=/Script/OrganMechanics.CharacterAttributeSet:Experience,AttributeOwner=\"/Script/CoreUObject.Class'/Script/OrganMechanics.CharacterAttributeSet'\")" (Math|Conversions|ToFloat(Integer) (Variables|Default|GetEXPGained)))
  (Actor|DestroyActor))