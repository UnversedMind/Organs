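; Base interactable actor that modifies the player's gameplay attributes when used, as an instant, single-shot interaction that is always available.
; BeginPlay creates a title/description widget with the actor as its data model, fed name and description through property bridges.
; Interact applies each AttributesToModify entry to player 0's Ability System Component, posting a notification for one specific attribute.
; The DestroyActor node is unconnected, so the actor persists after use.
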(event Custom|OnInteract
  (bind _attributestomodify (Variables|Default|GetAttributesToModify))
  (bind _keys (Utilities|Map|Keys _attributestomodify))
  (for _array_element _keys
    (Class|GameplayEffectExtender|ApplyModifier (Ability|GetAbilitySystemComponent (Game|GetPlayerCharacter 0)) _array_element (.Value (Utilities|Map|Find _attributestomodify _array_element)))
    (if (== _array_element "(AttributeName=\"Experience\",Attribute=/Script/OrganMechanics.CharacterAttributeSet:Experience,AttributeOwner=\"/Script/CoreUObject.Class'/Script/OrganMechanics.CharacterAttributeSet'\")")
      (Class|NotificationManagerSubsystem|AddNotification (Subsystems|GetNotificationManagerSubsystem) "Value" (Utilities|String|ToString(Float) (.Value (Utilities|Map|Find _attributestomodify _array_element)))))))

(event EventBeginPlay
  (|CallParentFunction)
  (bind _returnvalue (UserInterface|CreateWidget "/Game/Organs5/UI/Common/WB_GenericWidgetTitleDescription.WB_GenericWidgetTitleDescription_C"))
  (UserInterface|SetWidget (Variables|Default|GetWidget) _returnvalue)
  (Class|WidgetView|SetDataModel _returnvalue self))

(fn ConstructionScript)

(fn CanUserInteract
  (return true))

(fn GetControls
  (return 0))

(fn GetData
  (bind _returnvalue (Class|StringPropertyBridge|CreatePropertyBridge (Utilities|String|ToString(Text) (Variables|Default|GetInteractableName))))
  (bind _returnvalue_2 (Class|StringPropertyBridge|CreatePropertyBridge (Utilities|String|ToString(Text) (Variables|Default|GetInteractableDescription))))
  (bind _returnvalue_3 (Class|ArrayPropertyBridge|CreatePropertyBridge (Utilities|Array|MakeArray _returnvalue _returnvalue_2)))
  (return _returnvalue_3))

(fn GetInteractionTime
  (return 0.0))

(fn Interact
  (CallFunction|OnInteract)
  (return true))

(fn IsSingleShotInteraction
  (return true))

(fn StopInteract
  (return false))