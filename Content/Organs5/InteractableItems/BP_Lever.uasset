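; BP_Lever is an interactable lever that toggles between two positions with an instant, single-shot interaction.
; Each Interact call runs LevelInteraction, which plays or reverses the LevelAngle timeline according to InOnPosition, then flips that flag.
; The timeline update lerps the pitch of RotationAngle between LevelAngles and its negative to swing the lever.
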(fn ConstructionScript)

(fn LevelInteraction
  (bind _levelangle (Variables|Default|GetLevelAngle))
  (if (Variables|Default|GetinOnPosition)
    (Utilities|String|Reverse _levelangle)
    (else
      (Audio|Components|Audio|Play _levelangle)))
  (Variables|Default|SetinOnPosition (not (Variables|Default|GetinOnPosition))))

(fn CanUserInteract
  (return true))

(fn GetInteractionTime
  (return 0.0))

(fn Interact
  (CallFunction|LevelInteraction)
  (return true))

(fn IsSingleShotInteraction
  (return true))

(fn StopInteract
  (return false))