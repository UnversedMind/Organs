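; BP_InventoryItem is an interactable pickup that puts its item into the player's inventory.
; Interacting is instant and single-shot: it adds ItemName to the next available slot of the first player character's InventoryComponent.
; PostInteract then destroys the actor.
; GetData exposes the interactable's name and description as property bridges, while GetControls returns nothing and interaction is always allowed.
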(event EventPostInteract
  (Actor|DestroyActor))

(fn ConstructionScript)

(fn CanUserInteract
  (return true))

(fn GetControls
  (return 0))

(fn GetData
  (bind _returnvalue (Class|StringPropertyBridge|CreatePropertyBridge (Utilities|String|ToString(Text) (Variables|Default|GetInteractableName))))
  (bind _returnvalue_2 (Class|StringPropertyBridge|CreatePropertyBridge (Utilities|String|ToString(Text) (Variables|Default|GetInteractableDescription))))
  (bind _returnvalue_3 (Class|ArrayPropertyBridge|CreatePropertyBridge (Utilities|Array|MakeArray _returnvalue _returnvalue_2)))
  (return _returnvalue_3))

(fn GetInteractionTime
  (return 0.0))

(fn Interact
  (Class|InventoryComponent|AddItemtoInventoryatNextAvailableSlot (Actor|GetComponentbyClass (Game|GetPlayerCharacter 0) "/Script/InventorySystem.InventoryComponent") (Variables|Default|GetItem%20Name))
  (return true))

(fn IsSingleShotInteraction
  (return true))

(fn StopInteract
  (return true))