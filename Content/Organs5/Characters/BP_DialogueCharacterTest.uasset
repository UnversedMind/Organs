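; A test dialogue character that the player can interact with at any time, instantly and repeatedly, to start a conversation.
; Interact passes its Dialogue data to the DialogueSubsystem, adds a WB_DialogueUI widget to the viewport, layers the UI input mapping context and blends the view to this actor.
; StopInteract removes that mapping context and blends the view back to the player character, without removing the widget itself.
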(fn ConstructionScript)

(fn CanUserInteract
  (return true))

(fn GetInteractionTime
  (return 0.0))

(fn Interact
  (bind _returnvalue (Game|GetPlayerController 0))
  (bind _returnvalue_2 (PlayerController|LocalPlayerSubsystems|GetEnhancedInputLocalPlayerSubsystem _returnvalue))
  (Class|DialogueSubsystem|AcceptDialogue (Subsystems|GetDialogueSubsystem) (Variables|/Script/DialogueSystem.DialogueComponent|GetDialogue (Variables|Default|GetDialogue)))
  (bind _returnvalue_3 (UserInterface|CreateWidget "/Game/Organs5/UI/WB_DialogueUI.WB_DialogueUI_C"))
  (UserInterface|Viewport|AddtoViewport _returnvalue_3 0)
  (Utilities|IsValid _returnvalue_2
    (:Is%20Valid
      (Input|AddMappingContext _returnvalue_2 "/Game/Organs5/Input/IMC_UI.IMC_UI" 10 "(bIgnoreAllPressedKeysUntilRelease=True,bForceImmediately=False,bNotifyUserSettings=False)"))
    (:Is%20Not%20Valid
      _))
  (Game|Player|SetViewTargetwithBlend (Game|GetPlayerController 0) self 1.0 "VTBlend_Linear" 0.0 true)
  (return true))

(fn IsSingleShotInteraction
  (return false))

(fn StopInteract
  (bind _returnvalue (Game|GetPlayerController 0))
  (bind _returnvalue_2 (PlayerController|LocalPlayerSubsystems|GetEnhancedInputLocalPlayerSubsystem _returnvalue))
  (Utilities|IsValid _returnvalue_2
    (:Is%20Valid
      (Input|RemoveMappingContext _returnvalue_2 "/Game/Organs5/Input/IMC_UI.IMC_UI" "(bIgnoreAllPressedKeysUntilRelease=True,bForceImmediately=False,bNotifyUserSettings=False)"))
    (:Is%20Not%20Valid
      _))
  (Game|Player|SetViewTargetwithBlend (Game|GetPlayerController 0) (Game|GetPlayerCharacter 0) 1.0 "VTBlend_Linear" 0.0 true)
  (return true))